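; BP_Cassette is a clickable cassette actor that expects a BP_CassetteManager as its parent actor.
; On BeginPlay it writes its Name into the W_CharacterCassette widgets on its side and top.
; Clicking the mesh toggles Loaded, calling Select or Unload on the manager with a fixed index of zero.
; Cursor hover applies an outline overlay material with no matching clear, and its own Load and Unload events are empty.
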(event OnClicked(SM_Cassette)
  (params (TouchedComponent :type Primitive%20Component%20Object%20Reference) (ButtonPressed :type Key%20Structure :default "None"))
  (if (not (Variables|Default|GetLoaded))
    (bind _asbp_cassette_manager (Utilities|Casting|CastToBP_CassetteManager (Actor|GetParentActor)))
    (Default|Select _asbp_cassette_manager)
    (Variables|Default|SetLoaded true)
    (else
      (bind _asbp_cassette_manager_2 (Utilities|Casting|CastToBP_CassetteManager (Actor|GetParentActor)))
      (Default|Unload _asbp_cassette_manager_2)
      (Variables|Default|SetLoaded false))))

(event OnBeginCursorOver(SM_Cassette)
  (params (TouchedComponent :type Primitive%20Component%20Object%20Reference))
  (Rendering|Material|SetOverlayMaterial (Variables|Default|GetSM_Cassette) "/Game/M_Outline.M_Outline" false 0 :!class /Script/Engine.MeshComponent))

(event Custom|Load)

(event Custom|Unload)

(event EventBeginPlay
  (bind _asw_character_cassette (Utilities|Casting|CastToW_CharacterCassette (UserInterface|GetWidget (Variables|Default|GetNameSide))))
  (Variables|/Script/UMG.TextBlock|SetText (Variables|/Game/W_CharacterCassette.W_CharacterCassette_C|GetTB_Name _asw_character_cassette) (Utilities|Text|ToText(Name) (Variables|Default|GetName)))
  (bind _asw_character_cassette_2 (Utilities|Casting|CastToW_CharacterCassette (UserInterface|GetWidget (Variables|Default|GetNameTop))))
  (Variables|/Script/UMG.TextBlock|SetText (Variables|/Game/W_CharacterCassette.W_CharacterCassette_C|GetTB_Name _asw_character_cassette_2) (Utilities|Text|ToText(Name) (Variables|Default|GetName))))

(fn ConstructionScript)