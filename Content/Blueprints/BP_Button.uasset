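; BP_Button is a clickable 3D menu button whose ButtonFunction enum sets its text label in the construction script.
; Cursor hover and click events on the mesh offset the actor vertically from its starting location to mimic pressing.
; Clicking then blends the player's view to the matching section camera, with Shop also spawning ShopBox items after a delay.
; Quit gets a label but has no click action.
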(event OnBeginCursorOver(StaticMesh)
  (params (TouchedComponent :type Primitive%20Component%20Object%20Reference))
  (bind _buttonlocation (Variables|Default|GetButtonLocation))
  (Transformation|SetActorLocation (Math|Vector|MakeVector (.x _buttonlocation) (.y _buttonlocation) (- (.z _buttonlocation) 2.0)) false false))

(event OnEndCursorOver(StaticMesh)
  (params (TouchedComponent :type Primitive%20Component%20Object%20Reference))
  (bind _buttonlocation (Variables|Default|GetButtonLocation))
  (Transformation|SetActorLocation (Math|Vector|MakeVector (.x _buttonlocation) (.y _buttonlocation) (.z _buttonlocation)) false false))

(event OnClicked(StaticMesh)
  (params (TouchedComponent :type Primitive%20Component%20Object%20Reference) (ButtonPressed :type Key%20Structure :default "None"))
  (bind _returnvalue (Game|GetPlayerController 0))
  (bind _buttonlocation (Variables|Default|GetButtonLocation))
  (bind _buttonlocation_2 (Variables|Default|GetButtonLocation))
  (Transformation|SetActorLocation (Math|Vector|MakeVector (.x _buttonlocation_2) (.y _buttonlocation_2) (- (.z _buttonlocation_2) 9.0)) false false)
  (Utilities|FlowControl|Delay 0.2)
  (Transformation|SetActorLocation (Math|Vector|MakeVector (.x _buttonlocation) (.y _buttonlocation) (- (.z _buttonlocation) 7.0)) false false)
  (switch Utilities|FlowControl|Switch|SwitchonENUM_ButtonFunction (Variables|Default|GetButtonFunction)
    (:NewEnumerator0
      (Game|Player|SetViewTargetwithBlend (Game|GetPlayerController 0) (Variables|Default|GetFrontCam) 0.5 "VTBlend_Linear" 0.0 false))
    (:NewEnumerator4
      (Game|Player|SetViewTargetwithBlend _returnvalue (Variables|Default|GetQuestsCam) 0.5 "VTBlend_Linear" 0.0 false))
    (:NewEnumerator5
      (Game|Player|SetViewTargetwithBlend _returnvalue (Variables|Default|GetShopCam) 0.5 "VTBlend_Linear" 0.0 false)
      (Utilities|FlowControl|Delay 0.7)
      (Default|SpawnItems (Variables|Default|GetShopBox)))
    (:NewEnumerator1
      (Game|Player|SetViewTargetwithBlend (Game|GetPlayerController 0) (Variables|Default|GetUnlocksCam) 0.5 "VTBlend_Linear" 0.0 false))
    (:NewEnumerator2
      (Game|Player|SetViewTargetwithBlend (Game|GetPlayerController 0) (Variables|Default|GetSettingsCam) 0.5 "VTBlend_Linear" 0.0 false))))

(event EventBeginPlay
  (Variables|Default|SetButtonLocation (Transformation|GetActorLocation)))

(fn ConstructionScript
  (bind _textrender (Variables|Default|GetTextRender))
  (switch Utilities|FlowControl|Switch|SwitchonENUM_ButtonFunction (Variables|Default|GetButtonFunction)
    (:NewEnumerator0
      (Rendering|Components|TextRender|SetText _textrender (Utilities|Text|FormatText "Play")))
    (:NewEnumerator4
      (Rendering|Components|TextRender|SetText _textrender (Utilities|Text|FormatText "Quests")))
    (:NewEnumerator5
      (Rendering|Components|TextRender|SetText _textrender (Utilities|Text|FormatText "Shop")))
    (:NewEnumerator1
      (Rendering|Components|TextRender|SetText _textrender (Utilities|Text|FormatText "Unlocks")))
    (:NewEnumerator2
      (Rendering|Components|TextRender|SetText _textrender (Utilities|Text|FormatText "Settings")))
    (:NewEnumerator3
      (Rendering|Components|TextRender|SetText _textrender (Utilities|Text|FormatText "Quit")))))