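; BP_ShopBox is a clickable shop actor that switches the player's view to a shop camera and spawns its items.
; BeginPlay caches six slot component locations; clicking the box blends to ShopCam, waits briefly, then calls SpawnItems.
; Behind a DoOnce, a delayed loop over ShopItems spawns generic BP_ShopItem actors one by one above matching slots, storing them in ShopItemActors.
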(event OnClicked(Box)
  (params (TouchedComponent :type Primitive%20Component%20Object%20Reference) (ButtonPressed :type Key%20Structure :default "None"))
  (Game|Player|SetViewTargetwithBlend (Game|GetPlayerController 0) (Variables|Default|GetShopCam) 0.5 "VTBlend_Linear" 0.0 false)
  (Utilities|FlowControl|Delay 0.7)
  (CallFunction|SpawnItems))

(event Custom|Spawn%20Items
  (Utilities|FlowControl|DoOnce false
    (:Completed
      (bind _array_index (Utilities|ForEachwithDelay (Variables|Default|GetShopItems) 0.2)
        (:Loop%20Body
          (bind _returnvalue (Game|SpawnActorfromClass "/Game/Blueprints/BP_ShopItem.BP_ShopItem_C" (Math|Transform|MakeTransform (Math|Vector|MakeVector (.x (Utilities|Array|Get(acopy) (Variables|Default|GetItemSlots) _array_index)) (.y (Utilities|Array|Get(acopy) (Variables|Default|GetItemSlots) _array_index)) (+ (.z (Utilities|Array|Get(acopy) (Variables|Default|GetItemSlots) _array_index)) 3e+02)) "0.000000,30.000000,0.000000" "1.000000,1.000000,1.000000") "Undefined" "MultiplyWithRoot" 0 0))
          (Utilities|Array|Add (Variables|Default|GetShopItemActors) _returnvalue))))))

(event EventBeginPlay
  (Utilities|Array|Add (Variables|Default|GetItemSlots) (Transformation|GetWorldLocation (Variables|Default|GetItemSlot1)))
  (Utilities|Array|Add (Variables|Default|GetItemSlots) (Transformation|GetWorldLocation (Variables|Default|GetItemSlot2)))
  (Utilities|Array|Add (Variables|Default|GetItemSlots) (Transformation|GetWorldLocation (Variables|Default|GetItemSlot3)))
  (Utilities|Array|Add (Variables|Default|GetItemSlots) (Transformation|GetWorldLocation (Variables|Default|GetItemSlot4)))
  (Utilities|Array|Add (Variables|Default|GetItemSlots) (Transformation|GetWorldLocation (Variables|Default|GetItemSlot5)))
  (Utilities|Array|Add (Variables|Default|GetItemSlots) (Transformation|GetWorldLocation (Variables|Default|GetItemSlot6))))

(fn ConstructionScript)