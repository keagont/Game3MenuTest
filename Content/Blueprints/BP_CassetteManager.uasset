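; BP_CassetteManager spawns the selectable cassettes and tracks which one is selected.
; On BeginPlay it spawns a vertically stacked BP_Cassette for each unlocked entry, passing itself and the index, and stores each reference back in the array.
; Select unloads the previous cassette when the stored index is below a hardcoded limit, then records the new one.
; Enable moves the manager to a fixed location; Hide, Load and FullyLoad are empty.
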(event Custom|Hide)

(event Custom|Enable
  (Transformation|SetActorLocation "350.000000,430.000000,310.000000" false false))

(event Custom|Load)

(event Custom|Unload
  (params (CassetteIndex :type Integer))
  (Default|Unload (.CassetteBP (Utilities|Struct|BreakST_CharacterCassette (Utilities|Array|Get(acopy) (Variables|Default|GetCassettes) CassetteIndex)))))

(event Custom|Select
  (params (CassetteIndex :type Integer))
  (if (< (Variables|Default|GetSelectedCassette) 9)
    (CallFunction|Unload (Variables|Default|GetSelectedCassette))
    (Variables|Default|SetSelectedCassette CassetteIndex)
    (else
      (Variables|Default|SetSelectedCassette CassetteIndex))))

(event Custom|FullyLoad)

(event Custom|SpawnCassettes
  (bind _returnvalue (Transformation|GetActorRotation))
  (bind _returnvalue_2 (Transformation|GetActorLocation))
  (for (_array_element _array_index) (Variables|Default|GetCassettes)
    (if (.Unlocked (Utilities|Struct|BreakST_CharacterCassette _array_element))
      (bind _returnvalue_3 (Game|SpawnActorfromClass "/Game/Blueprints/BP_Cassette.BP_Cassette_C" (Math|Transform|MakeTransform (Math|Vector|MakeVector (.x _returnvalue_2) (- (.y _returnvalue_2) 9.0) (+ (.z _returnvalue_2) 1.8e+02 (* _array_index -20))) (Math|Rotator|MakeRotator 9e+01 (.pitch _returnvalue) (.yaw _returnvalue)) "1.000000,1.000000,1.000000") "Undefined" "MultiplyWithRoot" 0 (.Name (Utilities|Struct|BreakST_CharacterCassette _array_element)) self _array_index 0))
      (Utilities|Array|SetArrayElem (Variables|Default|GetCassettes) _array_index (Utilities|Struct|MakeST_CharacterCassette (.Name (Utilities|Struct|BreakST_CharacterCassette _array_element)) (.Unlocked (Utilities|Struct|BreakST_CharacterCassette _array_element)) _returnvalue_3)))))

(event EventBeginPlay
  (CallFunction|SpawnCassettes)
  (Variables|Default|SetSelectedCassette (Utilities|Array|Length (Variables|Default|GetCassettes))))

(fn ConstructionScript)