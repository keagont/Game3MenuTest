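; BP_Eject is a clickable 3D button actor that switches the player's view to a top camera.
; It caches its location on BeginPlay and nudges itself along Y while the cursor hovers over its static mesh, restoring it when the cursor leaves.
; Clicking the mesh blends the player controller's view target to TopCam.
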(event OnBeginCursorOver(StaticMesh)
  (params (TouchedComponent :type Primitive%20Component%20Object%20Reference))
  (bind _buttonlocation (Variables|Default|GetButtonLocation))
  (Transformation|SetActorLocation (Math|Vector|MakeVector (.x _buttonlocation) (- (.y _buttonlocation) 3.0) (.z _buttonlocation)) false false))

(event OnEndCursorOver(StaticMesh)
  (params (TouchedComponent :type Primitive%20Component%20Object%20Reference))
  (bind _buttonlocation (Variables|Default|GetButtonLocation))
  (Transformation|SetActorLocation (Math|Vector|MakeVector (.x _buttonlocation) (.y _buttonlocation) (.z _buttonlocation)) false false))

(event OnClicked(StaticMesh)
  (params (TouchedComponent :type Primitive%20Component%20Object%20Reference) (ButtonPressed :type Key%20Structure :default "None"))
  (Game|Player|SetViewTargetwithBlend (Game|GetPlayerController 0) (Variables|Default|GetTopCam) 0.5 "VTBlend_Linear" 0.0 false))

(event EventBeginPlay
  (Variables|Default|SetButtonLocation (Transformation|GetActorLocation)))

(fn ConstructionScript)