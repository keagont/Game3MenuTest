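; BP_LevelSlider is a clickable slider actor that steps a Slider component between preset positions.
; Each click increments SlideBarIndex, wrapping it by Slots, then snaps the Slider to the relative location of one of three SlidePoint components.
; Any index without its own position falls back to the first point.
; Click and hover events also print debug text; the index drives nothing else here.
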(event OnClicked(Slider)
  (params (TouchedComponent :type Primitive%20Component%20Object%20Reference) (ButtonPressed :type Key%20Structure :default "None"))
  (Development|PrintText "Clicking!!")
  (bind _output_get (Variables|Default|SetSlideBarIndex (Math|Integer|%(Integer) (+ (Variables|Default|GetSlideBarIndex) 1) (Variables|Default|GetSlots))))
  (switch int _output_get
    (:Default
      (Transformation|SetRelativeLocation (Variables|Default|GetSlider) (Variables|/Script/Engine.SceneComponent|GetRelativeLocation (Variables|Default|GetSlidePoint1)) false false :!label _label))
    (:0
      (goto _label))
    (:1
      (Transformation|SetRelativeLocation (Variables|Default|GetSlider) (Variables|/Script/Engine.SceneComponent|GetRelativeLocation (Variables|Default|GetSlidePoint2)) false false))
    (:2
      (Transformation|SetRelativeLocation (Variables|Default|GetSlider) (Variables|/Script/Engine.SceneComponent|GetRelativeLocation (Variables|Default|GetSlidePoint3)) false false))))

(event OnBeginCursorOver(Slider)
  (params (TouchedComponent :type Primitive%20Component%20Object%20Reference))
  (Development|PrintText "Hovering!"))

(fn ConstructionScript)