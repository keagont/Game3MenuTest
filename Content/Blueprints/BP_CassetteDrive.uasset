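; BP_CassetteDrive is a clickable cassette drive door whose mesh tilts to show Closed, Open and Loaded states.
; Clicks cycle through the states with a brief overshoot-and-settle rotation, and cursor hover nudges the angle as feedback.
; Clicking while Open tells the CassetteManager to load, closing from Loaded only prints a level-loading message, and an Unload event swings the door back open.
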(event OnBeginCursorOver(StaticMesh)
  (params (TouchedComponent :type Primitive%20Component%20Object%20Reference))
  (switch Utilities|FlowControl|Switch|SwitchonENUM_CassetteSlotState (Variables|Default|GetState)
    (:NewEnumerator0
      (Transformation|SetWorldRotation (Variables|Default|GetStaticMesh) "0.000000,0.000000,2.000000" false false))
    (:NewEnumerator1
      (Transformation|SetWorldRotation (Variables|Default|GetStaticMesh) "0.000000,0.000000,38.000000" false false))
    (:NewEnumerator2
      (Transformation|SetWorldRotation (Variables|Default|GetStaticMesh) "0.000000,0.000000,4.000000" false false))))

(event OnEndCursorOver(StaticMesh)
  (params (TouchedComponent :type Primitive%20Component%20Object%20Reference))
  (switch Utilities|FlowControl|Switch|SwitchonENUM_CassetteSlotState (Variables|Default|GetState)
    (:NewEnumerator0
      (Transformation|SetWorldRotation (Variables|Default|GetStaticMesh) "0, 0, 0" false false))
    (:NewEnumerator1
      (Transformation|SetWorldRotation (Variables|Default|GetStaticMesh) "0.000000,0.000000,40.000000" false false))
    (:NewEnumerator2
      (Transformation|SetWorldRotation (Variables|Default|GetStaticMesh) "0.000000,0.000000,10.000000" false false))))

(event OnClicked(StaticMesh)
  (params (TouchedComponent :type Primitive%20Component%20Object%20Reference) (ButtonPressed :type Key%20Structure :default "None"))
  (bind _staticmesh (Variables|Default|GetStaticMesh))
  (bind _staticmesh_2 (Variables|Default|GetStaticMesh))
  (bind _staticmesh_3 (Variables|Default|GetStaticMesh))
  (switch Utilities|FlowControl|Switch|SwitchonENUM_CassetteSlotState (Variables|Default|GetState)
    (:NewEnumerator0
      (Transformation|SetWorldRotation _staticmesh_3 "0.000000,0.000000,45.000000" false false)
      (Utilities|FlowControl|Delay 0.2)
      (Transformation|SetWorldRotation _staticmesh_3 "0.000000,0.000000,40.000000" false false)
      (Variables|Default|SetState "NewEnumerator1"))
    (:NewEnumerator1
      (Transformation|SetWorldRotation _staticmesh_2 "0.000000,0.000000,8.000000" false false)
      (Default|Load (Variables|Default|GetCassetteManager))
      (Utilities|FlowControl|Delay 0.2)
      (Transformation|SetWorldRotation _staticmesh_2 "0.000000,0.000000,10.000000" false false)
      (Variables|Default|SetState "NewEnumerator2"))
    (:NewEnumerator2
      (Transformation|SetWorldRotation _staticmesh "0.000000,0.000000,-2.000000" false false)
      (Utilities|FlowControl|Delay 0.2)
      (Transformation|SetWorldRotation _staticmesh "0, 0, 0" false false)
      (Variables|Default|SetState "NewEnumerator0")
      (Development|PrintText "Loading Level"))))

(event Custom|Unload
  (bind _staticmesh (Variables|Default|GetStaticMesh))
  (Transformation|SetWorldRotation _staticmesh "0.000000,0.000000,45.000000" false false)
  (Utilities|FlowControl|Delay 0.2)
  (Transformation|SetWorldRotation _staticmesh "0.000000,0.000000,40.000000" false false)
  (Variables|Default|SetState "NewEnumerator1"))

(fn ConstructionScript)