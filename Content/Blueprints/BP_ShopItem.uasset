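; BP_ShopItem is a shop item actor that animates into place when play begins.
; BeginPlay records the actor's height, then plays SpawnTimeline to drive the animation.
; Its position track lerps the actor's Z from below up to the recorded height, while its rotation track tilts the Item component in roll and pitch together.
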(event EventBeginPlay
  (bind _returnvalue (Transformation|GetActorLocation))
  (Variables|Default|SetStartHeight (.z (Transformation|GetActorLocation)))
  (bind (_direction _positiontrack _rotationtrack) (Timeline|SpawnTimeline Play)
    (:Update
      (Transformation|SetActorLocation (Math|Vector|MakeVector (.x _returnvalue) (.y _returnvalue) (Math|Float|Lerp (- (Variables|Default|GetStartHeight) 3e+02) (Variables|Default|GetStartHeight) _positiontrack)) false false)
      (Transformation|SetRelativeRotation (Variables|Default|GetItem) (Math|Rotator|MakeRotator (Math|Float|Lerp -15.0 15.0 _rotationtrack) (Math|Float|Lerp -15.0 15.0 _rotationtrack) 0.0) false false))))

(fn ConstructionScript)