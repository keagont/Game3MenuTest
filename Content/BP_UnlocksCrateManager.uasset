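; BP_UnlocksCrateManager is an actor that runs a carousel of unlock crates browsed with back and next arrow buttons.
; On BeginPlay it links both child-actor arrows to itself and spawns crates from BoxesST at three slot locations.
; GoNext and GoBack shift the slot parent, reposition crates and update the active index.
; SetActiveBox activates that crate, but DisableInactiveBoxes then deactivates the same index, not the others.
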(event Custom|GoNext
  (if (< (Variables|Default|GetActiveIndex) (- (Utilities|Array|Length (Variables|Default|GetBoxesST)) 1))
    (Transformation|AddLocalOffset (Variables|Default|GetSlotsParent) "-300.000000,0.000000,0.000000" false false)
    (Variables|Default|SetActiveIndex (+ (Variables|Default|GetActiveIndex) 1))
    (CallFunction|SetActiveBox)
    (CallFunction|SetItemSlotLoc)
    (CallFunction|UpdateBoxLocs)))

(event Custom|GoBack
  (if (> (Variables|Default|GetActiveIndex) 0)
    (Transformation|AddLocalOffset (Variables|Default|GetSlotsParent) "300.000000,0.000000,0.000000" false false)
    (Variables|Default|SetActiveIndex (- (Variables|Default|GetActiveIndex) 1))
    (CallFunction|SetActiveBox)
    (CallFunction|SetItemSlotLoc)
    (CallFunction|UpdateBoxLocs)))

(event Custom|SpawnBoxes
  (for (_array_element _array_index) (Variables|Default|GetBoxesST)
    (bind _returnvalue (Game|SpawnActorfromClass "/Game/BP_UnlocksCrate.BP_UnlocksCrate_C" (Math|Transform|MakeTransform (Utilities|Array|Get(acopy) (Variables|Default|GetItemSlots) _array_index) "0, 0, 0" "1.000000,1.000000,1.000000") "Undefined" "MultiplyWithRoot" 0 (Utilities|Struct|BreakST_Boxes _array_element) 0))
    (Utilities|Array|Add (Variables|Default|GetBoxesBP) _returnvalue)))

(event Custom|SetActiveBox
  (Default|SetActive (Utilities|Array|Get(acopy) (Variables|Default|GetBoxesBP) (Variables|Default|GetActiveIndex)))
  (CallFunction|DisableInactiveBoxes))

(event Custom|DisableInactiveBoxes
  (for (_array_element _array_index) (Variables|Default|GetBoxesBP)
    (if (== _array_index (Variables|Default|GetActiveIndex))
      (Default|SetInactive _array_element))))

(event Custom|SetItemSlotLoc
  (Utilities|Array|SetArrayElem (Variables|Default|GetItemSlots) 0 (Transformation|GetWorldLocation (Variables|Default|GetBoxSlot1)))
  (Utilities|Array|SetArrayElem (Variables|Default|GetItemSlots) 1 (Transformation|GetWorldLocation (Variables|Default|GetBoxSlot2)))
  (Utilities|Array|SetArrayElem (Variables|Default|GetItemSlots) 2 (Transformation|GetWorldLocation (Variables|Default|GetBoxSlot3))))

(event Custom|UpdateBoxLocs
  (for (_array_element _array_index) (Variables|Default|GetBoxesBP)
    (Transformation|SetActorLocation _array_element (Utilities|Array|Get(acopy) (Variables|Default|GetItemSlots) _array_index) false false)))

(event EventBeginPlay
  (Utilities|FlowControl|Sequence
    (:then_0
      (bind _asbp_arrow_buttons (Utilities|Casting|CastToBP_ArrowButtons (Variables|/Script/Engine.ChildActorComponent|GetChildActor (Variables|Default|GetBackArrow))))
      (Variables|/Game/BP_ArrowButtons.BP_ArrowButtons_C|SetNextArrow _asbp_arrow_buttons false)
      (Variables|/Game/BP_ArrowButtons.BP_ArrowButtons_C|SetManager _asbp_arrow_buttons self))
    (:then_1
      (bind _asbp_arrow_buttons_2 (Utilities|Casting|CastToBP_ArrowButtons (Variables|/Script/Engine.ChildActorComponent|GetChildActor (Variables|Default|GetNextArrow))))
      (Variables|/Game/BP_ArrowButtons.BP_ArrowButtons_C|SetNextArrow _asbp_arrow_buttons_2 true)
      (Variables|/Game/BP_ArrowButtons.BP_ArrowButtons_C|SetManager _asbp_arrow_buttons_2 self))
    (:then_2
      (CallFunction|SetItemSlotLoc)
      (CallFunction|SpawnBoxes))
    (:then_3
      (Variables|Default|SetActiveIndex 0)
      (CallFunction|SetActiveBox))))

(fn ConstructionScript)